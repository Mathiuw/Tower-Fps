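; BP_Weapon is an interactable world weapon pickup that grants a weapon to the actor interacting with it.
; The construction script sets its mesh from a weapon stats data asset.
; On interaction, it checks for a weapon inventory component, then adds its weapon data object to that inventory and to the owner.
; If none is assigned, it constructs one at runtime with max ammo, and it destroys itself after a successful pickup.
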(event `/Game/PSX/Blueprint/BPI_Interact.Interact`
  (params (interactor :type "Actor Object Reference"))
  (`self.WeaponPickup` interactor))

(fn `UserConstructionScript`
  (`/Engine/EditorBlueprintResources/StandardMacros.IsValid` (`self.weaponStatsDA`)
    (:`Is Valid`
      (`StaticMeshComponent.SetStaticMesh` (`self.StaticMesh`) (`/Game/PSX/DataAssset/WeaponStats/DA_WeaponStats.staticMesh` (`self.weaponStatsDA`))))
    (:`Is Not Valid`
      (`KismetSystemLibrary.PrintString` "No weaponStatsDA attached" true true (struct :`R` 1.0 :`G` 0.013091 :`A` 1.0)))))

(fn `WeaponPickup`
  (params (weaponOwner :type "Actor Object Reference"))
  (locals (`weapon inventory` :type "/Game/PSX/Blueprint/BPC_Inventory_Weapon Object Reference"))
  (bind _returnvalue (`self.GetComponentByClass` weaponOwner "/Game/PSX/Blueprint/BPC_Inventory_Weapon.BPC_Inventory_Weapon_C"))
  (bind _weaponowner (`local.weaponOwner`))
  (bind _weaponstatsda (`self.weaponStatsDA`))
  (bind _weaponda (`self.weaponDA`))
  ; check interacted actor have weapon inventory
  (`/Engine/EditorBlueprintResources/StandardMacros.IsValid` _returnvalue
    (:`Is Valid`
      (set `local.weapon inventory` _returnvalue)
      ; Case weapon DA is null, create one from scratch
      (`/Engine/EditorBlueprintResources/StandardMacros.IsValid` (`self.weaponDA`)
        (:`Is Valid`
          ; Add weapon to player
          (`/Game/PSX/Blueprint/BPC_Inventory_Weapon.WeaponAddToArray` (`local.weapon inventory`) _weaponda)
          (`AddComponent|NODE_AddBPC_Weapon-1` :`self` _weaponowner :`weapon` _weaponda))
        (:`Is Not Valid`
          (bind _returnvalue_2 (`|GenericCreateObject` "/Game/PSX/DataAssset/Items/DA_Item_Weapon.DA_Item_Weapon_C" _weaponstatsda (`/Game/PSX/DataAssset/WeaponStats/DA_WeaponStats.maxAmmo` _weaponstatsda)))
          (`/Game/PSX/Blueprint/BPC_Inventory_Weapon.WeaponAddToArray` (`local.weapon inventory`) _returnvalue_2)
          (`AddComponent|NODE_AddBPC_Weapon-0` :`self` _weaponowner :`weapon` _returnvalue_2)))
      (`KismetSystemLibrary.PrintString` "Weapon component added" true true (struct :`R` 0.027454 :`G` 1.0 :`A` 1.0))
      (`self.K2_DestroyActor`))
    (:`Is Not Valid`
      (`KismetSystemLibrary.PrintString` "Actor does not have weapon inventory" true true (struct :`R` 1.0 :`G` 0.013091 :`A` 1.0)))))