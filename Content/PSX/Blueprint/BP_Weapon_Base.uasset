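; Base Blueprint for a world weapon pickup that an interactor collects through the Interact event.
; WeaponPickup looks up the interactor's BPC_Inventory_Weapon component and, unless the inventory is full, adds this weapon's DataAsset to its array.
; It then calls AddBPCWeapon on the owner and destroys the pickup actor, with debug prints reporting the full and success cases.
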(event `/Game/PSX/Blueprint/BPI_Interact.Interact`
  (params (interactor :type "Actor Object Reference"))
  (`self.WeaponPickup` interactor))

(fn `UserConstructionScript`)

(fn `WeaponPickup`
  (params (weaponOwner :type "Actor Object Reference"))
  (bind _returnvalue (`self.GetComponentByClass` weaponOwner "/Game/PSX/Blueprint/BPC_Inventory_Weapon.BPC_Inventory_Weapon_C"))
  ; Is inventory full?
  (`/Engine/EditorBlueprintResources/StandardMacros.IsValid` _returnvalue
    (:`Is Valid`
      (if (`/Game/PSX/Blueprint/BPC_Inventory_Weapon.IsInventoryFull?` _returnvalue)
        (`KismetSystemLibrary.PrintString` "Inventory full")
        (else
          ; Add weapon to player
          (`/Game/PSX/Blueprint/BPC_Inventory_Weapon.WeaponAddToArray` _returnvalue (`self.dataAsset`))
          (`AddComponent|NODE_AddBPC_Weapon-0` :`self` (`local.weaponOwner`))
          (`KismetSystemLibrary.PrintString` "Weapon component added" true true (struct :`R` 0.027454 :`G` 1.0 :`A` 1.0))
          (`self.K2_DestroyActor`))))))