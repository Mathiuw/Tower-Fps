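; Inventory component that stores a player pawn's weapons in a size-limited array and tracks ammo totals for small, large and shell types.
; It adds an Enhanced Input mapping context on BeginPlay, removes it on EndPlay, and binds switch and drop inputs.
; Dropping spawns a BP_Weapon from the selected data asset, removes the entry and calls WeaponSwitch, which only handles wrapping to index zero.
; Switch and drop fire event dispatchers.
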(event `self.ReceiveBeginPlay`
  ; Add Inventory Input if it is player
  (bind _returnvalue (`self.GetPlayerInputSubsystem`))
  (`EnhancedInputSubsystemInterface.AddMappingContext` _returnvalue "/Game/Input/IMC_Inventory.IMC_Inventory" 0 (struct)))

(event `self.ReceiveEndPlay`
  (params (EndPlayReason :type "EEndPlayReason Enum" :default "Destroyed"))
  ; Remove inventory input when distroyed
  (bind _aspawn (cast `Pawn` (`self.GetOwner`)))
  (bind _asplayer_controller (cast `PlayerController` (`Pawn.GetController` _aspawn)))
  (`EnhancedInputSubsystemInterface.RemoveMappingContext` (pcsubsystem `EnhancedInputLocalPlayerSubsystem` _asplayer_controller) "/Game/Input/IMC_Inventory.IMC_Inventory" (struct)))

(event `EnhancedInput|/Game/Input/Actions/IA_Inventory_Switch`
  (params (ActionValue :type "Float (double-precision)") (ElapsedSeconds :type "Float (double-precision)") (TriggeredSeconds :type "Float (double-precision)") (InputAction :type "InputAction Object Reference" :default "/Game/Input/Actions/IA_Inventory_Switch.IA_Inventory_Switch"))
  ; Switch Weapon Input
  (:`Started`
    (`self.WeaponSwitch` 0.0)))

(event `EnhancedInput|/Game/Input/Actions/IA_Inventory_Drop`
  (params (ActionValue :type Boolean) (ElapsedSeconds :type "Float (double-precision)") (TriggeredSeconds :type "Float (double-precision)") (InputAction :type "InputAction Object Reference" :default "/Game/Input/Actions/IA_Inventory_Drop.IA_Inventory_Drop"))
  ; Weapon Drop Input
  (:`Started`
    (`self.WeaponDrop`)))

(fn `AddAmmoByType`
  (params (ammoAmount :type Integer) (ammoType :type "/Game/PSX/DataAssset/WeaponStats/E_AmmoTypes Enum" :default "NewEnumerator0"))
  (switch `/Game/PSX/DataAssset/WeaponStats/E_AmmoTypes` ammoType
    (:`NewEnumerator0`
      (set `self.smallAmmoAmount` (+ (`self.smallAmmoAmount`) ammoAmount)))
    (:`NewEnumerator1`
      (set `self.largeAmmoAmount` (+ (`self.largeAmmoAmount`) ammoAmount)))
    (:`NewEnumerator2`
      (set `self.shellAmount` (+ (`self.shellAmount`) ammoAmount)))))

(fn `GetPlayerInputSubsystem`
  (returns (ReturnValue :type "EnhancedInputLocalPlayerSubsystem Object Reference"))
  (bind _aspawn (cast `Pawn` (`self.GetOwner`))
    (:`then`
      (bind _asplayer_controller (cast `PlayerController` (`Pawn.GetController` _aspawn))))
    (:`CastFailed`
      _))
  (return (pcsubsystem `EnhancedInputLocalPlayerSubsystem` _asplayer_controller)))

(fn `IsInventoryFull?`
  (returns (bool :type Boolean))
  (return (>= (`KismetArrayLibrary.Array_Length` (`self.weapons`)) (`self.inventorySize`))))

(fn `WeaponAddToArray`
  (params (`weapon DA` :type "/Game/PSX/DataAssset/Items/DA_Item_Weapon Object Reference"))
  ; Is inventory full?
  (if (`self.IsInventoryFull?`)
    (`KismetSystemLibrary.PrintString` "Inventory full")
    (else
      ; Add Weapon to Weapons Array
      (`KismetArrayLibrary.Array_Add` (`self.weapons`) (`local.weapon DA`))
      (`KismetSystemLibrary.PrintString` (`KismetStringLibrary.Concat_StrStr` (`/Game/PSX/DataAssset/Items/DA_Item_base.name` (`/Game/PSX/DataAssset/Items/DA_Item_Weapon.weaponStats` (`local.weapon DA`))) " added to weapon inventory array") true true (struct :`R` 0.089887 :`G` 1.0 :`A` 1.0)))))

(fn `WeaponDrop`
  (bind (_returnvalue_location _returnvalue_rotation) (`KismetMathLibrary.BreakTransform` (`Actor.GetTransform` (`self.GetOwner`))))
  (bind _output (`|GetArrayItem` (`self.weapons`) (`self.selectIndex`)))
  ; Spawn weapon actor
  (`/Engine/EditorBlueprintResources/StandardMacros.IsValid` _output
    (:`Is Valid`
      (`|SpawnActorFromClass` "/Game/PSX/Blueprint/BP_Weapon.BP_Weapon_C" (`KismetMathLibrary.MakeTransform` _returnvalue_location _returnvalue_rotation) "Undefined" "MultiplyWithRoot" null (`/Game/PSX/DataAssset/Items/DA_Item_Weapon.weaponStats` _output) _output null)
      ; Remove weapon from array
      (`KismetArrayLibrary.Array_Remove` (`self.weapons`) (`self.selectIndex`))
      (`KismetSystemLibrary.PrintString` "Dropped weapon" true true (struct :`R` 0.094314 :`G` 1.0 :`A` 1.0))
      ; Go to next weapon
      (`self.WeaponSwitch` 1.0)
      ; Call OnWeaponDrop Event
      (`self.OnWeaponDrop`))
    (:`Is Not Valid`
      (`KismetSystemLibrary.PrintString` "Doesnt have weapon" true true (struct :`R` 1.0 :`G` 0.014948 :`A` 1.0)))))

(fn `WeaponSwitch`
  (params (actionValue :type "Float (double-precision)"))
  ; Go to next or previous index, if the list is over, go back to the start
  (if (== (+ (`self.selectIndex`) actionValue) (`KismetArrayLibrary.Array_Length` (`self.weapons`)))
    (set `self.selectIndex` 0)
    ; Call OnWeaponSwitch Event
    (`self.OnWeaponSwitch`)
    (`KismetSystemLibrary.PrintString` "switched weapons" true true (struct :`G` 1.0 :`B` 0.042229 :`A` 1.0))))