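; Weapon component that gives its owner shoot and reload input and keeps the BP_Character_PSX weapon mesh in sync with its weapon inventory.
; On BeginPlay it finds BPC_Inventory_Weapon, loads the selected weapon's mesh and adds IMC_Weapon for player-controlled owners, removing it on EndPlay.
; The inventory's drop event unloads the weapon and destroys the component when no weapons remain.
; Shoot and reload are placeholders that only print debug messages.
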(event `EnhancedInput|/Game/Input/Actions/IA_Weapon_Reload`
  (params (ActionValue :type Boolean) (ElapsedSeconds :type "Float (double-precision)") (TriggeredSeconds :type "Float (double-precision)") (InputAction :type "InputAction Object Reference" :default "/Game/Input/Actions/IA_Weapon_Reload.IA_Weapon_Reload"))
  ; Weapon reload input
  (:`Started`
    (`self.Reload Weapon`)))

(event `EnhancedInput|/Game/Input/Actions/IA_Weapon_Shoot`
  (params (ActionValue :type Boolean) (ElapsedSeconds :type "Float (double-precision)") (TriggeredSeconds :type "Float (double-precision)") (InputAction :type "InputAction Object Reference" :default "/Game/Input/Actions/IA_Weapon_Shoot.IA_Weapon_Shoot"))
  ; Weapon shoot input
  (:`Started`
    (`self.ShootWeapon`)))

(event `self.ReceiveBeginPlay`
  (bind _weaponinventory (`self.weaponInventory`))
  (bind _returnvalue (`Actor.GetComponentByClass` (`self.GetOwner`) "/Game/PSX/Blueprint/BPC_Inventory_Weapon.BPC_Inventory_Weapon_C"))
  (`|ExecutionSequence`
    (:`then_0`
      ; Check if owned actor have weapon inventory and set to variable
      (`/Engine/EditorBlueprintResources/StandardMacros.IsValid` _returnvalue
        (:`Is Valid`
          (bind _output_get (set `self.weaponInventory` _returnvalue))
          (add `/Game/PSX/Blueprint/BPC_Inventory_Weapon.OnWeaponDrop` _output_get (delegate `WeaponDrop`))
          ; Load Weapon
          (bind _asbp_character_psx (cast `/Game/PSX/Blueprint/BP_Character_PSX` (`self.GetOwner`)))
          (`/Game/PSX/Blueprint/BP_Character_PSX.WeaponLoad` _asbp_character_psx (`/Game/PSX/DataAssset/DA_WeaponStats.skeletalMesh` (`|GetArrayItem` (`/Game/PSX/Blueprint/BPC_Inventory_Weapon.weapons` _weaponinventory) (`/Game/PSX/Blueprint/BPC_Inventory_Weapon.selectIndex` _weaponinventory)))))
        (:`Is Not Valid`
          (`KismetSystemLibrary.PrintString` "Pawn doesnt have weapon inventory " true true (struct :`R` 1.0 :`G` 0.00337 :`A` 1.0)))))
    (:`then_1`
      ; If owner pawn have player controller, add weapon input
      (bind _aspawn (cast `Pawn` (`self.GetOwner`)))
      (bind _asplayer_controller (cast `PlayerController` (`Pawn.GetController` _aspawn)))
      (`EnhancedInputSubsystemInterface.AddMappingContext` (pcsubsystem `EnhancedInputLocalPlayerSubsystem` _asplayer_controller) "/Game/Input/IMC_Weapon.IMC_Weapon" 0 (struct)))))

(event `WeaponDrop`
  ; Check if owned actor have weapon inventory and set to variable
  (`self.OnWeaponDropFunc`))

(event `self.ReceiveEndPlay`
  (params (EndPlayReason :type "EEndPlayReason Enum" :default "Destroyed"))
  ; Remove player weapon input when destroying
  (bind _aspawn (cast `Pawn` (`self.GetOwner`)))
  (bind _asplayer_controller (cast `PlayerController` (`Pawn.GetController` _aspawn)))
  (`EnhancedInputSubsystemInterface.RemoveMappingContext` (pcsubsystem `EnhancedInputLocalPlayerSubsystem` _asplayer_controller) "/Game/Input/IMC_Weapon.IMC_Weapon" (struct)))

(fn `OnWeaponDropFunc`
  ; Unload Weapon
  (bind _asbp_character_psx (cast `/Game/PSX/Blueprint/BP_Character_PSX` (`self.GetOwner`)))
  (`/Game/PSX/Blueprint/BP_Character_PSX.WeaponUnload` _asbp_character_psx)
  ; If weponInventory doesnt have weapons, delete component
  (if (== (`KismetArrayLibrary.Array_Length` (`/Game/PSX/Blueprint/BPC_Inventory_Weapon.weapons` (`self.weaponInventory`))) 0)
    (`self.K2_DestroyComponent`)))

(fn `Reload Weapon`
  (`KismetSystemLibrary.PrintString` "reloaded weapon" true true (struct :`R` 0.04539 :`G` 1.0 :`B` 0.001614 :`A` 1.0)))

(fn `ShootWeapon`
  (`KismetSystemLibrary.PrintString` "shot weapon" true true (struct :`R` 0.031064 :`G` 1.0 :`B` 0.003341 :`A` 1.0)))